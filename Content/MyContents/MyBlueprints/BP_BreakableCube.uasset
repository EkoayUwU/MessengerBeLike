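; BP_BreakableCube is a cube that the player breaks with repeated sword hits.
; Each SwordHit event resets the third-person character's JumpCount to zero and decrements the cube's LifeCount.
; The remaining life selects one of three materials on the static mesh to show its damage stage, and the actor destroys itself at zero.
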(event EventSwordHit
  ;[0.05 0.05 0.05] Cube Life
  (bind _asbp_third_person_character (Utilities|Casting|CastToBP_ThirdPersonCharacter (Game|GetPlayerCharacter 0)))
  (Variables|/Game/ThirdPerson/Blueprints/BP_ThirdPersonCharacter.BP_ThirdPersonCharacter_C|SetJumpCount _asbp_third_person_character 0)
  (bind _output_get (Variables|VariableConfig|SetLifeCount (- (Variables|VariableConfig|GetLifeCount) 1)))
  (switch int _output_get
    (:Default
      (Rendering|Material|SetMaterial (Variables|Default|GetStaticMeshComponent1) 0 "/Game/MyContents/MyMaterials/BreakableCube_1.BreakableCube_1"))
    (:1
      (Rendering|Material|SetMaterial (Variables|Default|GetStaticMeshComponent1) 0 "/Game/MyContents/MyMaterials/BreakableCube_3.BreakableCube_3"))
    (:2
      (Rendering|Material|SetMaterial (Variables|Default|GetStaticMeshComponent1) 0 "/Game/MyContents/MyMaterials/BreakableCube_2.BreakableCube_2")))
  (if (== (Variables|VariableConfig|GetLifeCount) 0)
    (Actor|DestroyActor)))

(fn ConstructionScript)